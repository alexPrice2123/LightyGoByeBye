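; Torch Blueprint whose point light dims as a countdown runs out.
; BeginPlay caches the light's intensity and falloff exponent, and AddLightTimer updates the target game time that sets the remaining time.
; Each Tick scales intensity by time left over MaxTime and raises the falloff exponent as that ratio drops.
; A reset event restores the cached values; the collider overlap handler is empty.
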(event `self.ReceiveBeginPlay`
  (`self.save light proprtites`))

(event `AddLightTimer`
  (params (`time(sec)` :type "Float (double-precision)"))
  (if (> (`self.TargetTime`) 0.0)
    (set `self.TargetTime` (+ (`KismetSystemLibrary.GetGameTimeInSeconds`) `time(sec)`))
    (else
      (set `self.TargetTime` (+ (`self.TargetTime`) `time(sec)`)))))

(event `CalcTimeLeft`
  (set `self.TimeLeft` (- (`self.TargetTime`) (`KismetSystemLibrary.GetGameTimeInSeconds`))))

(event `self.ReceiveTick`
  (params (DeltaSeconds :type "Float (single-precision)"))
  (`self.CalcTimeLeft`)
  (`LightComponent.SetIntensity` (`self.PointLight`) (* (`self.Light intensity`) (/ (`self.TimeLeft`) (`self.MaxTime`))))
  (`PointLightComponent.SetLightFalloffExponent` (`self.PointLight`) (- 16.0 (* 16.0 (/ (`self.TimeLeft`) (`self.MaxTime`))))))

(event `reset light`
  (`PointLightComponent.SetLightFalloffExponent` (`self.PointLight`) (`self.light falloff`))
  (`LightComponent.SetIntensity` (`self.PointLight`) (`self.Light intensity`)))

(event `save light proprtites`
  (bind _pointlight (`self.PointLight`))
  (set `self.light falloff` (`PointLightComponent.LightFalloffExponent` _pointlight))
  (set `self.Light intensity` (`LightComponentBase.Intensity` _pointlight)))

(event `self.Torch Collidor.OnComponentBeginOverlap`
  (params (OverlappedComponent :type "PrimitiveComponent Object Reference") (OtherActor :type "Actor Object Reference") (OtherComp :type "PrimitiveComponent Object Reference") (OtherBodyIndex :type Integer) (bFromSweep :type Boolean) (SweepResult :type "HitResult Structure (by ref)")))

(fn `UserConstructionScript`)