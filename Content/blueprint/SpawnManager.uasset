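; Spawn manager that scatters oil and key pickups across tagged spawn points when play begins.
; SpawnOil and SpawnKey each gather tagged Pawns as markers, then shuffle the list and spawn at the first entry's location on every loop pass.
; SpawnOil removes used points, but SpawnKey removes from OilActors, so key locations can repeat.
; Both loops call DestroyActor on the manager itself each pass.
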(event `self.ReceiveBeginPlay`
  (`self.SpawnOil` 25)
  (`self.SpawnKey` 8))

(event `self.ReceiveTick`
  (params (DeltaSeconds :type "Float (single-precision)")))

(event `keySpawn`)

(fn `SpawnKey`
  (params (`Spawn Number` :type Integer))
  (bind _key_actors (`self.key Actors`))
  (bind _returnvalue_location (`KismetMathLibrary.BreakTransform` (`self.GetTransform` (`|GetArrayItem` _key_actors))))
  (bind _outactors (`GameplayStatics.GetAllActorsOfClassWithTag` "/Script/Engine.Pawn" "keyspawn"))
  (set `self.key Actors` _outactors)
  (for _ (range `Spawn Number`)
    (`KismetArrayLibrary.Array_Shuffle` _key_actors)
    (`|SpawnActorFromClass` "/Game/keysstuff/Key_Blueprint1.Key_Blueprint1_C" (`KismetMathLibrary.MakeTransform` _returnvalue_location) "AlwaysSpawn" "MultiplyWithRoot" null null)
    (`KismetArrayLibrary.Array_Remove` (`self.oil Actors`))
    (`self.K2_DestroyActor`)))

(fn `SpawnOil`
  (params (`Spawn Number` :type Integer))
  (bind _oil_actors (`self.oil Actors`))
  (bind _returnvalue_location (`KismetMathLibrary.BreakTransform` (`self.GetTransform` (`|GetArrayItem` _oil_actors))))
  (bind _outactors (`GameplayStatics.GetAllActorsOfClassWithTag` "/Script/Engine.Pawn" "oilspawn"))
  (set `self.oil Actors` _outactors)
  (for _ (range `Spawn Number`)
    (`KismetArrayLibrary.Array_Shuffle` _oil_actors)
    (`|SpawnActorFromClass` "/Game/Oil_Blueprint.Oil_Blueprint_C" (`KismetMathLibrary.MakeTransform` _returnvalue_location) "AlwaysSpawn" "MultiplyWithRoot" null null)
    (`KismetArrayLibrary.Array_Remove` (`self.oil Actors`))
    (`self.K2_DestroyActor`)))

(fn `UserConstructionScript`)