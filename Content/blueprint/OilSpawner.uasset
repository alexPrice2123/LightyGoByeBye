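; OilSpawner scatters Key_Blueprint pickups across random spawn points once, when play begins.
; It gathers Pawns tagged "oilspawn", then repeatedly shuffles the list, spawns at the first entry's location and removes that entry to avoid reusing points.
; The loop count is fixed rather than based on the number of points found, and the spawner calls DestroyActor on itself inside the loop body.
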(event `self.ReceiveBeginPlay`
  (`self.OilSpawn`))

(event `self.ReceiveTick`
  (params (DeltaSeconds :type "Float (single-precision)")))

(event `OilSpawn`
  (bind _out_actors (`self.Out Actors`))
  (bind _returnvalue_location (`KismetMathLibrary.BreakTransform` (`self.GetTransform` (`|GetArrayItem` _out_actors))))
  (bind _outactors (`GameplayStatics.GetAllActorsOfClassWithTag` "/Script/Engine.Pawn" "oilspawn"))
  (set `self.Out Actors` _outactors)
  (for _ (range 16)
    (`KismetArrayLibrary.Array_Shuffle` _out_actors)
    (`|SpawnActorFromClass` "/Game/Key_Blueprint.Key_Blueprint_C" (`KismetMathLibrary.MakeTransform` _returnvalue_location) "AlwaysSpawn" "MultiplyWithRoot" null null)
    (`KismetArrayLibrary.Array_Remove` (`self.Out Actors`))
    (`self.K2_DestroyActor`)))

(fn `UserConstructionScript`)