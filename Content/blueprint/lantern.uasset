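; Lantern Blueprint with a point light that dims toward zero during play.
; BeginPlay saves the light's intensity and falloff exponent, which the resetlight event restores.
; Each Tick interpolates intensity down and drives the falloff exponent toward a higher target.
; The InterpSpeedCalc helper recomputes the dimming speed every frame from the remaining intensity over a time constant, so the fade slows as it darkens.
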(event `self.ReceiveBeginPlay`
  (`self.save light proprtites`))

(event `self.ReceiveTick`
  (params (DeltaSeconds :type "Float (single-precision)"))
  (bind _pointlight (`self.PointLight`))
  (bind _intensity (`LightComponentBase.Intensity` (`self.PointLight`)))
  (bind _interpspeed (`self.interpSpeedCalc` 10.0 _intensity))
  (`PointLightComponent.SetLightFalloffExponent` _pointlight (`KismetMathLibrary.FInterpTo` (`PointLightComponent.LightFalloffExponent` (`self.PointLight`)) 16.0 DeltaSeconds))
  (`LightComponent.SetIntensity` _pointlight (`KismetMathLibrary.FInterpTo` _intensity 0.0 DeltaSeconds _interpspeed)))

(event `reset light`
  (`PointLightComponent.SetLightFalloffExponent` (`self.PointLight`) (`self.light falloff`))
  (`LightComponent.SetIntensity` (`self.PointLight`) (`self.Light intensity`)))

(event `save light proprtites`
  (bind _pointlight (`self.PointLight`))
  (set `self.light falloff` (`PointLightComponent.LightFalloffExponent` _pointlight))
  (set `self.Light intensity` (`LightComponentBase.Intensity` _pointlight)))

(fn `interpSpeedCalc`
  (params (Time :type "Float (double-precision)") (Current :type "Float (double-precision)") (Target :type "Float (double-precision)"))
  (returns (InterpSpeed :type "Float (double-precision)"))
  (return (/ (`KismetMathLibrary.Abs` (- (`KismetMathLibrary.Abs` Current) (`KismetMathLibrary.Abs` Target))) Time)))

(fn `UserConstructionScript`)