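; BP_Monster is an AI monster that hunts the first-person player and kills on contact.
; Delay-throttled Tick logic plays heartbeats at the player when a visibility trace is unblocked, then wanders slowly while the player's LightSource is above zero, otherwise chases fast.
; Sighting a pawn also sends it toward the player.
; Box overlap sets Dead and runs timelines that tilt and shift the camera, move the lantern and alter post-processing.
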(event `self.Vision.OnSeePawn`
  (params (Pawn :type "Pawn Object Reference"))
  (`self.FollowPawn`))

(event `self.ReceiveTick`
  (params (DeltaSeconds :type "Float (single-precision)"))
  (bind _returnvalue (`GameplayStatics.GetPlayerCharacter` 0))
  (bind _charactermovement (`self.CharacterMovement`))
  (bind _returnvalue_location (`KismetMathLibrary.BreakTransform` (`self.GetTransform` (`GameplayStatics.GetPlayerCharacter` 0))))
  (`KismetSystemLibrary.Delay` 1.2)
  (bind _outhit (`KismetSystemLibrary.LineTraceSingle` :`Start` (`self.K2_GetActorLocation`) :`End` (`self.K2_GetActorLocation` (`GameplayStatics.GetPlayerCharacter` 0)) :`TraceChannel` "TraceTypeQuery1" :`DrawTime` 1.0))
  (if (not (`GameplayStatics.BreakHitResult` _outhit))
    (`GameplayStatics.PlaySoundAtLocation` "/Game/Sounds/HeartBeats.HeartBeats" (`self.K2_GetActorLocation` _returnvalue) (struct) 0.5 1.0 0.0 null null _returnvalue null))
  (`KismetSystemLibrary.Delay` 3.0)
  (bind _asbp_first_person_character (cast `/Game/FirstPerson/Blueprints/BP_FirstPersonCharacter` (`GameplayStatics.GetPlayerCharacter` 0)))
  (if (> (`/Game/FirstPerson/Blueprints/BP_FirstPersonCharacter.LightSource` _asbp_first_person_character) 0.0)
    (set `CharacterMovementComponent.MaxWalkSpeed` 300.0 _charactermovement)
    (if (not (> (`KismetMathLibrary.VSize` (`MovementComponent.Velocity` (`self.CharacterMovement`))) 0.0))
      (set `self.RandomPoint` (`NavigationSystemV1.K2_GetRandomReachablePointInRadius` (`self.K2_GetActorLocation`) 10000.0 null null))
      (`|AIMoveTo` self (`self.RandomPoint`) null 1000.0))
    (else
      (set `CharacterMovementComponent.MaxWalkSpeed` 1000.0 _charactermovement)
      (`|AIMoveTo` self _returnvalue_location null 100.0))))

(event `FollowPawn`
  (bind _returnvalue_location (`KismetMathLibrary.BreakTransform` (`self.GetTransform` (`GameplayStatics.GetPlayerCharacter` 0))))
  (`|AIMoveTo` self _returnvalue_location null 100.0))

(event `self.ReceiveBeginPlay`
  (`GameplayStatics.SpawnSoundAttached` "/Game/Sounds/Monster.Monster" (`self.Mesh`) "None" (0.0 0.0 0.0) (struct) "KeepRelativeOffset" false 1.0 1.0 0.0 null null))

(event `self.Box.OnComponentBeginOverlap`
  (params (OverlappedComponent :type "PrimitiveComponent Object Reference") (OtherActor :type "Actor Object Reference") (OtherComp :type "PrimitiveComponent Object Reference") (OtherBodyIndex :type Integer) (bFromSweep :type Boolean) (SweepResult :type "HitResult Structure (by ref)"))
  (bind _asbp_first_person_character (cast `/Game/FirstPerson/Blueprints/BP_FirstPersonCharacter` OtherActor))
  (set `/Game/FirstPerson/Blueprints/BP_FirstPersonCharacter.Dead` true _asbp_first_person_character)
  (bind (_direction _newtrack_0) (`Timeline|Timeline_1`)
    (:`Update`
      (bind _firstpersoncamera (`/Game/FirstPerson/Blueprints/BP_FirstPersonCharacter.FirstPersonCamera` _asbp_first_person_character))
      (`SceneComponent.K2_SetRelativeRotation` _firstpersoncamera (`KismetMathLibrary.MakeRotator` (* _newtrack_0 1.0)) false false)
      (`SceneComponent.K2_AddLocalOffset` _firstpersoncamera (`KismetMathLibrary.MakeVector` 0.0 (/ _newtrack_0 7.5) (/ _newtrack_0 12.0)) false false)
      (`/Engine/EditorBlueprintResources/StandardMacros.DoOnce` false
        (:`Completed`
          (bind (_direction_2 _newtrack_1) (`Timeline|Timeline_0`)
            (:`Update`
              (bind _returnvalue (* _newtrack_1 10.0))
              (`SceneComponent.K2_AddLocalOffset` (`/Game/FirstPerson/Blueprints/BP_FirstPersonCharacter.Lant` _asbp_first_person_character) (`KismetMathLibrary.MakeVector` _returnvalue _returnvalue _returnvalue) false false))
            (:`Finished`
              (bind (_direction_3 _newtrack_1_2) (`Timeline|Timeline`)
                (:`Update`
                  (set `CameraComponent.PostProcessSettings` (make `PostProcessSettings` :`ColorOffset` (`KismetMathLibrary.MakeVector4` _newtrack_1_2 _newtrack_1_2 _newtrack_1_2 _newtrack_1_2)) (`/Game/FirstPerson/Blueprints/BP_FirstPersonCharacter.FirstPersonCamera` _asbp_first_person_character)))))))))))

(fn `UserConstructionScript`)